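; Private child Blueprint of an RSP rendering tool that customizes how the path tracer restarts.
; RestartPathTracer switches to Lit mode if path tracing was last enabled, then calls the parent restart after a retriggerable delay.
; It then briefly toggles the visible-lights path tracing console variable on and off.
; Unconnected nodes showcase the FL library's rendering method and screenshot functions, alongside a disabled samples-per-pixel experiment.
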(event `self.ReceiveTick`
  (params (DeltaSeconds :type "Float (single-precision)"))
  ;[0 0 0 1 200] Tick
  (`parent.ReceiveTick` DeltaSeconds))

(event `self.ReceiveBeginPlay`
  ;[0 0 0 1 200] Begin Play
  (`parent.ReceiveBeginPlay`))

(event `self.RestartPathTracer`
  (params (WorldContextObject :type "Object Object Reference"))
  ;[0 0 0 1 200] Restart Path Tracer
  (`|ExecutionSequence`
    (:`then_0`
      (if (`self.PathTracerEnable_Last`)
        (`self.ShowLitMode`)))
    (:`then_1`
      (`KismetSystemLibrary.RetriggerableDelay` 0.6)
      (`parent.RestartPathTracer`)
      (`KismetSystemLibrary.ExecuteConsoleCommand` "r.PathTracing.VisibleLights 1" null)
      (`KismetSystemLibrary.Delay` 0.4)
      (`KismetSystemLibrary.ExecuteConsoleCommand` "r.PathTracing.VisibleLights 0" null))))

(fn `UserConstructionScript`)