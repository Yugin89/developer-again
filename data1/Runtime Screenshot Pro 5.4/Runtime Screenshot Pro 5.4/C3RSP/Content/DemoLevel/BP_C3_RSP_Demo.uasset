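; Demo Blueprint for an RSP screenshot and path-tracing toolset, driven by keyboard shortcuts.
; Z switches between raster and path tracing, while X toggles the path tracer directly.
; Other keys trigger instant or path-traced Lite, Pro and Ultra screenshots by multiplier or resolution, saved under random names in a hardcoded temp folder.
; BeginPlay adds the demo widget and binds the RSP manager's capture callback, which displays each captured texture in that widget.
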(event `Key|Z`
  (params (Key :type "Key Structure"))
  ;[0 0 0 1 60] Turn Path Tracer On/Off
  (:`Pressed`
    (`/Engine/EditorBlueprintResources/StandardMacros.FlipFlop`
      (:`A`
        ;;[0 0 0] #1 Set Rendering Method
        (`C3_RSP_FunctionLibrary.FL_SetRenderingMethod` "Raster"))
      (:`B`
        (`C3_RSP_FunctionLibrary.FL_SetRenderingMethod` "PathTracing")))))

(event `Key|X`
  (params (Key :type "Key Structure"))
  ;[0 0 0 1 60] Turn Path Tracer On/Off
  (:`Pressed`
    (bind _isa (`/Engine/EditorBlueprintResources/StandardMacros.FlipFlop`)
      (:`A`
        _)
      (:`B`
        _))
    ;;[0 0 0] Enable Render Feature Directly
    (`C3_RSP_FunctionLibrary.FL_EnablePathTracer` _isa)))

(event `Key|J`
  (params (Key :type "Key Structure"))
  ;[0 0 0 1 100] Path Tracer Screenshot Example
  ;;[0 0 0 1 60] Path Tracer Screenshot (Resolution)
  (:`Pressed`
    ;;;[0 0 0] Path Tracer Screenshot
    (`C3_RSP_FunctionLibrary.FL_PathTracerShot_Lite` (`KismetStringLibrary.Concat_StrStr` "D:\\_Temp2\\" (`C3_RSP_FunctionLibrary.FL_RandomString_Pro` 4)))))

(event `Key|C`
  (params (Key :type "Key Structure"))
  ;[0 0 0 1 100] Normal Screenshot Example
  ;;[0 0 0 1 60] Instant Shot (Multiplier)
  (:`Pressed`
    ;;;[0 0 0] Instant Screenshot
    (`C3_RSP_FunctionLibrary.FL_InstantScreenshot_Lite` (`KismetStringLibrary.Concat_StrStr` "D:\\_Temp2\\" (`C3_RSP_FunctionLibrary.FL_RandomString_Pro` 4)))))

(event `Key|K`
  (params (Key :type "Key Structure"))
  ;[0 0 0 1 100] Path Tracer Screenshot Example
  ;;[0 0 0 1 60] Path Tracer Screenshot (Resolution)
  (:`Pressed`
    ;;;[0 0 0] Path Tracer Screenshot
    (`C3_RSP_FunctionLibrary.FL_PathTracerShot_Pro` (`KismetStringLibrary.Concat_StrStr` "D:\\_Temp2\\" (`C3_RSP_FunctionLibrary.FL_RandomString_Pro` 4)) -1 1920 1080)))

(event `Key|V`
  (params (Key :type "Key Structure"))
  ;[0 0 0 1 100] Normal Screenshot Example
  ;;[0 0 0 1 60] Instant Shot (Multiplier)
  (:`Pressed`
    ;;;[0 0 0] Instant Screenshot
    (`C3_RSP_FunctionLibrary.FL_InstantScreenshot_Pro` (`KismetStringLibrary.Concat_StrStr` "D:\\_Temp2\\" (`C3_RSP_FunctionLibrary.FL_RandomString_Pro` 4)) 2)))

(event `Key|B`
  (params (Key :type "Key Structure"))
  ;[0 0 0 1 100] Normal Screenshot Example
  ;;[0 0 0 1 60] Instant Shot (Multiplier)
  (:`Pressed`
    ;;;[0 0 0] Instant Screenshot
    (`C3_RSP_FunctionLibrary.FL_InstantScreenshot_Ultra` (`KismetStringLibrary.Concat_StrStr` "D:\\_Temp2\\" (`C3_RSP_FunctionLibrary.FL_RandomString_Pro` 4)) false false 3)))

(event `Key|L`
  (params (Key :type "Key Structure"))
  ;[0 0 0 1 100] Path Tracer Screenshot Example
  ;;[0 0 0 1 60] Path Tracer Screenshot (Resolution)
  (:`Pressed`
    ;;;[0 0 0] Path Tracer Screenshot
    (`C3_RSP_FunctionLibrary.FL_PathTracerShot_Ultra` (`KismetStringLibrary.Concat_StrStr` "D:\\_Temp2\\" (`C3_RSP_FunctionLibrary.FL_RandomString_Pro` 4)) false false -1 3840 2160)))

(event `Key|N`
  (params (Key :type "Key Structure"))
  ;[0 0 0 1 100] Normal Screenshot Example
  ;;[0 0 0 1 60] Instant Shot (Resolution)
  (:`Pressed`
    ;;;[0 0 0] Instant Screenshot
    (`C3_RSP_FunctionLibrary.FL_InstantScreenshot_Pro` (`KismetStringLibrary.Concat_StrStr` "D:\\_Temp2\\" (`C3_RSP_FunctionLibrary.FL_RandomString_Pro` 4)) -1 1920 1080)))

(event `Key|F`
  (params (Key :type "Key Structure"))
  ;[0 0 0 1 100] Path Tracer Screenshot Example
  ;;[0 0 0 1 60] Path Tracer Screenshot (Multiplier)
  (:`Pressed`
    ;;;[0 0 0] Path Tracer Screenshot
    (`C3_RSP_FunctionLibrary.FL_PathTracerShot_Lite` (`KismetStringLibrary.Concat_StrStr` "D:\\_Temp2\\" (`C3_RSP_FunctionLibrary.FL_RandomString_Pro` 4)))))

(event `Key|M`
  (params (Key :type "Key Structure"))
  ;[0 0 0 1 100] Normal Screenshot Example
  ;;[0 0 0 1 60] Instant Shot (Resolution)
  (:`Pressed`
    ;;;[0 0 0] Instant Screenshot
    (`C3_RSP_FunctionLibrary.FL_InstantScreenshot_Ultra` (`KismetStringLibrary.Concat_StrStr` "D:\\_Temp2\\" (`C3_RSP_FunctionLibrary.FL_RandomString_Pro` 4)) false false -1 3840 2160)))

(event `Key|G`
  (params (Key :type "Key Structure"))
  ;[0 0 0 1 100] Path Tracer Screenshot Example
  ;;[0 0 0 1 60] Path Tracer Screenshot (Multiplier)
  (:`Pressed`
    ;;;[0 0 0] Path Tracer Screenshot
    (`C3_RSP_FunctionLibrary.FL_PathTracerShot_Pro` (`KismetStringLibrary.Concat_StrStr` "D:\\_Temp2\\" (`C3_RSP_FunctionLibrary.FL_RandomString_Pro` 4)) 2)))

(event `Key|H`
  (params (Key :type "Key Structure"))
  ;[0 0 0 1 100] Path Tracer Screenshot Example
  ;;[0 0 0 1 60] Path Tracer Screenshot (Multiplier)
  (:`Pressed`
    ;;;[0 0 0] Path Tracer Screenshot
    (`C3_RSP_FunctionLibrary.FL_PathTracerShot_Ultra` (`KismetStringLibrary.Concat_StrStr` "D:\\_Temp2\\" (`C3_RSP_FunctionLibrary.FL_RandomString_Pro` 4)) false false 3)))

(event `self.ReceiveBeginPlay`
  ;[0 0 0 1 60] On Screenshot Capture
  (bind _returnvalue (`|CreateWidget` "/C3_RSP/DemoLevel/WBP_C3_RSP_Demo.WBP_C3_RSP_Demo_C" (`GameplayStatics.GetPlayerController` 0)))
  (`UserWidget.AddToViewport` _returnvalue 0)
  (add `C3_RSP_ManagerBase.OnScreenshotCaptured` (`C3_RSP_FunctionLibrary.GetRSPManager`) (delegate `OnScreenshotCaptured_Event`)))

(event `OnScreenshotCaptured_Event`
  (params (SizeX :type Integer) (SizeY :type Integer) (Texture :type "Texture2D Object Reference") (RawData :type "Array of Color Structure (by ref)"))
  ;[0 0 0 1 60] On Screenshot Capture
  ;;[0 0 0] Show the new captured texture into screen
  (bind _foundwidgets (`WidgetBlueprintLibrary.GetAllWidgetsOfClass` "/C3_RSP/DemoLevel/WBP_C3_RSP_Demo.WBP_C3_RSP_Demo_C" false))
  (bind _output (`|GetArrayItem` _foundwidgets))
  (`/Engine/EditorBlueprintResources/StandardMacros.IsValid` _output
    (:`Is Valid`
      (`Image.SetBrushFromTexture` (`/C3_RSP/DemoLevel/WBP_C3_RSP_Demo.Image_0` _output) Texture false))))

(fn `UserConstructionScript`)