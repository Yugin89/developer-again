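; BP_WaterRiverSwim is a river water volume that serves the swim component and identifies itself as Unreal Water System water.
; On overlap begin and end, it sends enter and exit water volume messages to the other actor.
; Its volume info reports surface Z from the river spline point closest to the player, or the spline start without a valid player.
; It flags that Z for updating, disables the buoyancy helper and supplies swim priority and Z offset.
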(event `self.ReceiveActorBeginOverlap`
  (params (OtherActor :type "Actor Object Reference"))
  ;[0.0616 0.3004 1] These events serve the Swim component
  (message `/Game/SwimComponent/Blueprints/Interface/BPI_Swim.EnterWaterVolume` OtherActor self))

(event `self.ReceiveActorEndOverlap`
  (params (OtherActor :type "Actor Object Reference"))
  ;[0.0616 0.3004 1] These events serve the Swim component
  (message `/Game/SwimComponent/Blueprints/Interface/BPI_Swim.ExitWaterVolume` OtherActor self))

(fn `GetSwimComponent`
  (returns (swimComponent :type "/Game/SwimComponent/Blueprints/Component/BP_SwimComponent Object Reference"))
  (return null))

(fn `GetWaterVolumeInfo`
  (params (Player :type "Actor Object Reference"))
  (returns (ZLocationWaterVolume :type "Float (double-precision)") (IsUEWaterSystem :type Boolean) (CanUseBuoyancyHelperInThisArea :type Boolean) (UpdateZLocationCurrentWaterVolume :type Boolean) (Priority :type Integer) (OffsetZLocation :type "Float (double-precision)") (IsWater :type Boolean) (IsExclusionVolume :type Boolean))
  (bind _splinecomp (`self.SplineComp`))
  (bind _priorityswim (`self.PrioritySwim`))
  (bind _offsetzlocation (`self.OffsetZLocation`))
  (bind (_returnvalue_x _returnvalue_y _returnvalue_z) (`KismetMathLibrary.BreakVector` (`SplineComponent.GetLocationAtTime` _splinecomp 0.0 "World" false)))
  (bind (_returnvalue_x_2 _returnvalue_y_2 _returnvalue_z_2) (`KismetMathLibrary.BreakVector` (`SplineComponent.FindLocationClosestToWorldLocation` _splinecomp (`self.K2_GetActorLocation` Player) "World")))
  (`/Engine/EditorBlueprintResources/StandardMacros.IsValid` Player
    (:`Is Valid`
      (return _returnvalue_z_2 true false true _priorityswim _offsetzlocation true false))
    (:`Is Not Valid`
      (return _returnvalue_z true false true _priorityswim _offsetzlocation true false))))

(fn `UserConstructionScript`)