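; BP_WaterExclusionVolume is a placeable volume that marks an exclusion area for the swim component's water system.
; Overlap begin and end on VolumeCollision send enter and exit water volume messages to the other actor, passing itself.
; GetWaterVolumeInfo flags it as an exclusion volume, with all other water settings zero or false.
; As a level-design helper, its construction script snaps it to a referenced WaterExclusionVolume's transform, then clears the reference.
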(event `self.VolumeCollision.OnComponentBeginOverlap`
  (params (OverlappedComponent :type "PrimitiveComponent Object Reference") (OtherActor :type "Actor Object Reference") (OtherComp :type "PrimitiveComponent Object Reference") (OtherBodyIndex :type Integer) (bFromSweep :type Boolean) (SweepResult :type "HitResult Structure (by ref)"))
  (message `/Game/SwimComponent/Blueprints/Interface/BPI_Swim.EnterWaterVolume` OtherActor self))

(event `self.VolumeCollision.OnComponentEndOverlap`
  (params (OverlappedComponent :type "PrimitiveComponent Object Reference") (OtherActor :type "Actor Object Reference") (OtherComp :type "PrimitiveComponent Object Reference") (OtherBodyIndex :type Integer))
  (message `/Game/SwimComponent/Blueprints/Interface/BPI_Swim.ExitWaterVolume` OtherActor self))

(fn `GetSwimComponent`
  (returns (swimComponent :type "/Game/SwimComponent/Blueprints/Component/BP_SwimComponent Object Reference"))
  (return null))

(fn `GetWaterVolumeInfo`
  (params (Player :type "Actor Object Reference"))
  (returns (ZLocationWaterVolume :type "Float (double-precision)") (IsUEWaterSystem :type Boolean) (CanUseBuoyancyHelperInThisArea :type Boolean) (UpdateZLocationCurrentWaterVolume :type Boolean) (Priority :type Integer) (OffsetZLocation :type "Float (double-precision)") (IsExclusionVolume :type Boolean))
  (return 0.0 false false false 0 0.0 true))

(fn `UserConstructionScript`
  ;[1 1 1] Helper for level designer
  (bind _waterexclusionvolume (`self.WaterExclusionVolume`)
    (:`then`
      (`self.K2_SetActorTransform` (`self.GetTransform` _waterexclusionvolume) false true)
      (set `self.WaterExclusionVolume` null))
    (:`else`)))