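; Helper actor in the swim component that tracks a target actor in XY, with forward and right offsets, to sample water surface info.
; Its Buoyancy component serves only as a water query.
; Each tick it teleports to the offset point, setting Z from its initial height minus water depth, capped at the target's height.
; It also re-enables the Buoyancy component's tick to work around a bug between water bodies.
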(event `self.ReceiveTick`
  (params (DeltaSeconds :type "Float (single-precision)"))
  (bind (_initiallocation_x _initiallocation_y _initiallocation_z) (`KismetMathLibrary.BreakVector` (`self.InitialLocation`)))
  (bind _buoyancy (`self.Buoyancy`))
  (bind _returnvalue (- _initiallocation_z (`self.Out Water Depth`)))
  ;[1 1 1] Fix bug between water bodies
  (if (not (`ActorComponent.IsComponentTickEnabled` _buoyancy))
    (`ActorComponent.SetComponentTickEnabled` _buoyancy true))
  ;[1 1 1] We can set our buoyancy component without buoyancy cause all we need is the surface info
  (bind _actortofollowxy (`self.ActorToFollowXY`)
    (:`then`
      (bind (_outwaterplanelocation _outwaterplanenormal _outwatersurfaceposition _outwaterdepth) (`BuoyancyComponent.GetLastWaterSurfaceInfo` (`self.Buoyancy`)))
      (set `self.Out Water Plane Normal` _outwaterplanenormal)
      (set `self.Out Water Surface Position` _outwatersurfaceposition)
      (set `self.Out Water Plane Location` _outwaterplanelocation)
      (set `self.Out Water Depth` _outwaterdepth)
      (bind _returnvalue_2 (`self.K2_GetActorRotation` _actortofollowxy))
      (bind (_returnvalue_x _returnvalue_y _returnvalue_z) (`KismetMathLibrary.BreakVector` (`self.K2_GetActorLocation` _actortofollowxy)))
      (bind (_returnvalue_x_2 _returnvalue_y_2) (`KismetMathLibrary.BreakVector` (+ (+ (* (`KismetMathLibrary.GetForwardVector` _returnvalue_2) (`self.OffsetForwardActor`)) (* (`KismetMathLibrary.GetRightVector` _returnvalue_2) (`self.OffsetRightActor`))) (`KismetMathLibrary.MakeVector` _returnvalue_x _returnvalue_y _returnvalue_z))))
      (`self.K2_SetActorLocation` (+ (`KismetMathLibrary.MakeVector` _returnvalue_x_2 _returnvalue_y_2) (`KismetMathLibrary.MakeVector` 0.0 0.0 (`KismetMathLibrary.FClamp` _returnvalue _returnvalue _returnvalue_z))) false true))
    (:`else`)))

(fn `UserConstructionScript`)